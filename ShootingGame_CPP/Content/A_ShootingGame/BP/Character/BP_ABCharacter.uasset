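; Player character Blueprint for a shooting game, with a socket-attached weapon and a prototype hitscan shot.
; BeginPlay spawns an owned actor, but sets the weapon reference NewVar0 to None before using it to disable physics and collision and attach to WeponSocket.
; Left click line-traces from the weapon's Muzzle socket along the weapon actor's forward vector, with debug drawing.
; Hits only print the bone name; no damage is applied.
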(event EventBeginPlay
  (Game|SpawnActorfromClass (Variables|Default|GetClass) (Math|Transform|MakeTransform "0, 0, 0" "0, 0, 0" "1,1,1") "Undefined" self 0)
  (bind _output_get (Variables|Default|SetNewVar_0 0))
  (Physics|SetSimulatePhysics (Variables|/Script/ShootingGame_CPP.Weapon|GetWeapon _output_get) false)
  (Collision|SetCollisionEnabled (Variables|/Script/ShootingGame_CPP.Weapon|GetWeapon _output_get) "NoCollision")
  (Transformation|AttachComponentToComponent (Variables|/Script/ShootingGame_CPP.Weapon|GetWeapon _output_get) (Variables|Character|GetMesh) "WeponSocket" "SnapToTarget" "SnapToTarget" "KeepRelative" true))

(event Input|ActionEvents|InputActionClickedLeft
  (params (Key :type Key%20Structure :default "None"))
  (bind _newvar_0 (Variables|Default|GetNewVar_0))
  (bind _weapon (Variables|/Script/ShootingGame_CPP.Weapon|GetWeapon _newvar_0))
  (bind _returnvalue (Transformation|GetSocketLocation _weapon "Muzzle"))
  (:Pressed
    (bind (_outhit _returnvalue_2) (Collision|LineTraceForObjects _returnvalue (+ _returnvalue (* (Math|Vector|GetForwardVector (Transformation|GetActorRotation _newvar_0)) 1e+03)) (Utilities|Array|MakeArray "ObjectTypeQuery1" "ObjectTypeQuery4" "ObjectTypeQuery3" "ObjectTypeQuery5" "ObjectTypeQuery6") true 0 "ForDuration"))
    (if _returnvalue_2
      (Development|PrintString (Utilities|String|ToString(Name) (.HitBoneName (Collision|BreakHitResult _outhit)))))))

(fn ConstructionScript)